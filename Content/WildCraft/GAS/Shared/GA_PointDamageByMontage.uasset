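; Gameplay ability that plays a montage and applies point damage when a tagged gameplay event arrives during it.
; After committing, it starts the configurable montage and listens for the listener tag, including child tags.
; Each event supplies target, causer, hit result and controller (via OptionalObject); damage is skipped without a controller.
; The ability ends on montage blend-out, interruption or cancellation, or when the commit fails.
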(event Ability|EventActivateAbility
  (|CallParentFunction)
  (bind _returnvalue (Ability|CommitAbility))
  (if _returnvalue
    (|PlayMontageandWaitProxy "None" (Variables|Default|GetMontageToPlay) (Variables|Default|GetMontagePlaySpeed) "None" true 1.0
      (:then
        (bind _payload (Ability|Tasks|WaitGameplayEvent (Variables|Default|GetListenerTag) 0 false false)
          (:EventReceived
            (bind _ascontroller (Utilities|Casting|CastToController (.OptionalObject (Utilities|Struct|BreakGameplayEventData _payload))))
            (Game|Damage|ApplyPointDamage (.Target (Utilities|Struct|BreakGameplayEventData _payload)) (Variables|Default|GetDamageCoefficient) (.ImpactNormal (Collision|BreakHitResult (Class|AbilitySystemBlueprintLibrary|EffectContextGetHitResult (.ContextHandle (Utilities|Struct|BreakGameplayEventData _payload))))) (Class|AbilitySystemBlueprintLibrary|EffectContextGetHitResult (.ContextHandle (Utilities|Struct|BreakGameplayEventData _payload))) _ascontroller (.Instigator (Utilities|Struct|BreakGameplayEventData _payload)) (Variables|Default|GetDamageType)))))
      (:OnBlendOut
        (Ability|EndAbility :!label _label))
      (:OnInterrupted
        (goto _label))
      (:OnCancelled
        (goto _label)))
    (else
      (Ability|EndAbility))))

(event Ability|EventOnEndAbility
  (params (bWasCancelled :type Boolean))
  (|CallParentFunction bWasCancelled) ; 지금 이 노드는 비활성 상태입니다. \n핀을 끌어서 다른 노드를 연결하면 활성화됩니다.
)